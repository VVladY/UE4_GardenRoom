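; BP_Door is a double door that the player toggles open and closed with the F key while near it.
; Trigger overlaps enable and disable input for player controller 0, without checking which actor overlaps.
; The OpenDoors timeline drives the yaw of both door leaves, playing to open and reversing to close.
; Tick derives DoorIsClosed from the left door's timeline rotation to choose the direction.
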(event `self.Trigger.OnComponentBeginOverlap`
  (params (OtherActor :type "Actor Object Reference") (OtherComp :type "PrimitiveComponent Object Reference") (OtherBodyIndex :type Integer) (bFromSweep :type Boolean) (SweepResult :type "HitResult Structure (by ref)"))
  (`self.EnableInput` (`GameplayStatics.GetPlayerController` 0)))

(event `self.Trigger.OnComponentEndOverlap`
  (params (OtherActor :type "Actor Object Reference") (OtherComp :type "PrimitiveComponent Object Reference") (OtherBodyIndex :type Integer))
  (`self.DisableInput` (`GameplayStatics.GetPlayerController` 0)))

(event `Key|F`
  (params (Key :type "Key Structure" :default "AnyKey"))
  (:`Pressed`
    (if (`self.DoorIsClosed`)
      (bind (_direction _leftdoorrotation _rightdoorrotation) (`Timeline|OpenDoors` :!label _label)
        (:`Update`
          (`SceneComponent.K2_SetRelativeRotation` (`self.DoorRight`) (`KismetMathLibrary.MakeRotator` 0.0 0.0 _rightdoorrotation) false false)
          (`SceneComponent.K2_SetRelativeRotation` (`self.DoorLeft`) (`KismetMathLibrary.MakeRotator` 0.0 0.0 _leftdoorrotation) false false)))
      (else
        (goto _label :!via `Reverse`)))))

(event `self.ReceiveTick`
  (params (DeltaSeconds :type "Float (single-precision)"))
  (set `self.DoorIsClosed` (< (stale `Key|F` _leftdoorrotation) 1.0)))

(fn `UserConstructionScript`)